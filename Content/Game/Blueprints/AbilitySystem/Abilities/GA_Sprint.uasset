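; Gameplay ability that makes the owning character sprint while the input is held.
; On activation it reads the SprintSpeed row from the DT_MovementSpeed data table and sends it to the owner through SetMovementSpeedMessage.
; On input release it checks the owned tags for Crouching, restores either the CrouchedSpeed or MoveSpeed row, then ends the ability.
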(event `self.K2_ActivateAbility`
  (bind (_owneractor _avataractor _playercontroller _abilitysystemcomponent) (break `GameplayAbilityActorInfo` (`self.GetActorInfo`)))
  (bind _returnvalue (`|GetDataTableRow` "/Game/Game/misc/DT_MovementSpeed.DT_MovementSpeed" "SprintSpeed")
    (:`then`
      (message `/Game/Game/Blueprints/Interfaces/BPI_CharacterAbility.SetMovementSpeed` _owneractor (break `/Game/Game/Blueprints/Structs/FMovementSpeed` _returnvalue))
      (`AbilityTask_WaitInputRelease.WaitInputRelease` false
        (:`OnRelease`
          (bind _tagcontainer (message `GameplayTagAssetInterface.GetOwnedGameplayTags` _abilitysystemcomponent))
          (if (`BlueprintGameplayTagLibrary.HasTag` _tagcontainer (struct :`TagName` "Character.Status.Crouching"))
            (bind _returnvalue_2 (`|GetDataTableRow` "/Game/Game/misc/DT_MovementSpeed.DT_MovementSpeed" "CrouchedSpeed")
              (:`then`
                (message `/Game/Game/Blueprints/Interfaces/BPI_CharacterAbility.SetMovementSpeed` _owneractor (break `/Game/Game/Blueprints/Structs/FMovementSpeed` _returnvalue_2))))
            (else
              (bind _returnvalue_3 (`|GetDataTableRow` "/Game/Game/misc/DT_MovementSpeed.DT_MovementSpeed" "MoveSpeed")
                (:`then`
                  (message `/Game/Game/Blueprints/Interfaces/BPI_CharacterAbility.SetMovementSpeed` _owneractor (break `/Game/Game/Blueprints/Structs/FMovementSpeed` _returnvalue_3))))))
          (`self.K2_EndAbility`))))))