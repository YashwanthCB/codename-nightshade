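; GA_jump is a Gameplay Ability that handles the owning character's jump and hands off to ledge grabbing.
; On activation it asks the owner for a final ledge vector and sends a LedgeGrab gameplay event when that vector is non-zero.
; It also waits for input: press jumps with a velocity read from a speed-based curve, and release stops jumping and ends the ability.
; Cancellation also stops the jump; a Mantle event branch exists but is unconnected.
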(event `self.K2_ActivateAbility`
  (bind (_returnvalue_owneractor _returnvalue_avataractor _returnvalue_playercontroller _returnvalue_abilitysystemcomponent _returnvalue_skeletalmeshcomponent _returnvalue_animinstance _returnvalue_movementcomponent) (break `GameplayAbilityActorInfo` (`self.GetActorInfo`)))
  (bind _returnvalue_owneractor_2 (break `GameplayAbilityActorInfo` (`self.GetActorInfo`)))
  (bind _output_get (set `self.Owner Actor` _returnvalue_owneractor_2))
  (bind _ascapsule_collision (cast `CapsuleComponent` (`Actor.RootComponent` _output_get)))
  (set `self.Owner Capsule Collision` _ascapsule_collision)
  (bind _returnvalue (message `CharacterAbilityHelperInterface.GetFinalLedgeVector` (`self.Owner Actor`)))
  (set `self.FinalLedge` _returnvalue)
  (`|ExecutionSequence`
    (:`then_0`
      (if (!= (`self.FinalLedge`) (0.0 0.0 0.0))
        (`AbilitySystemBlueprintLibrary.SendGameplayEventToActor` (`self.Owner Actor`) (struct :`TagName` "Character.Status.LedgeGrab") (make `GameplayEventData` (struct) null null null null (struct) (struct :`GameplayTags` (struct :`(TagName` "Character.State.jump")))))))
    (:`then_1`
      (`|ExecutionSequence`
        (:`then_0`
          (`AbilityTask_WaitInputPress.WaitInputPress` false
            (:`OnPress`
              (bind _ascharacter_movement_component (cast `CharacterMovementComponent` _returnvalue_movementcomponent))
              (set `CharacterMovementComponent.JumpZVelocity` (`CurveFloat.GetFloatValue` (`self.JumpVelocityFloat`) (`KismetMathLibrary.VSize` (`Actor.GetVelocity` (`self.Owner Actor`)))) _ascharacter_movement_component)
              (set `CharacterMovementComponent.bNotifyApex` true _ascharacter_movement_component)
              (bind _ascharacter (cast `Character` (`self.Owner Actor`)))
              (`Character.Jump` _ascharacter))))
        (:`then_1`
          (`AbilityTask_WaitInputRelease.WaitInputRelease` false
            (:`OnRelease`
              (bind _ascharacter_2 (cast `Character` (`self.Owner Actor`))
                (:`then`
                  (`Character.StopJumping` _ascharacter_2)
                  (`self.K2_EndAbility`))
                (:`CastFailed`
                  (`KismetSystemLibrary.PrintString` "cast failed GA_jump" false))))))))))

(event `self.K2_OnEndAbility`
  (params (bWasCancelled :type Boolean))
  (if bWasCancelled
    (bind _ascharacter (cast `Character` (`self.Owner Actor`))
      (:`then`
        (`Character.StopJumping` _ascharacter)
        (`self.K2_EndAbility`))
      (:`CastFailed`
        (`KismetSystemLibrary.PrintString` "cast failed GA_jump" false)))))