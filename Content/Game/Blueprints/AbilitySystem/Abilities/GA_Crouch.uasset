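; GA_Crouch is a crouch gameplay ability that smoothly resizes a capsule collision to a target crouched half-height.
; CrouchInterpolate uses FInterpTo with world delta seconds and InterpSpeed to step the half-height toward the target, updating overlaps.
; When the interpolated value is within a small tolerance, it snaps the capsule to the target and ends the ability.
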(fn `CrouchInterpolate`
  (bind _returnvalue (`KismetMathLibrary.FInterpTo` (`CapsuleComponent.CapsuleHalfHeight` (`self.As Capsule Collision`)) (`self.TargetCrouchedHalfHeight`) (`GameplayStatics.GetWorldDeltaSeconds`) (`self.Interp Speed`)))
  (`CapsuleComponent.SetCapsuleHalfHeight` (`self.As Capsule Collision`) _returnvalue true)
  (if (`KismetMathLibrary.NearlyEqual_FloatFloat` _returnvalue (`self.TargetCrouchedHalfHeight`) 1.0)
    (`CapsuleComponent.SetCapsuleHalfHeight` (`self.As Capsule Collision`) (`self.TargetCrouchedHalfHeight`) true)
    (`self.K2_EndAbility`)))