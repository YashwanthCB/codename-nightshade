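; BP_NoiseMakingComponent is an unfinished component meant to let its owning actor make noise.
; MakeNoise sphere-overlaps for Pawns within NoiseRadius of the owner, excluding the owner, and loops over the results.
; The loop body is empty, so no pawn is notified.
; The Intensity input, an AI controller lookup and a debug sphere draw are left unused or disconnected.
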(fn `MakeNoise`
  (params (Intensity :type "Float (double-precision)"))
  (bind (_outactors _returnvalue) (`KismetSystemLibrary.SphereOverlapActors` (`Actor.K2_GetActorLocation` (`self.GetOwner`)) (`self.NoiseRadius`) (`|MakeArray` "ObjectTypeQuery3" :!type "EObjectTypeQuery Enum") null (`|MakeArray` (`self.GetOwner`))))
  (if _returnvalue
    (for _array_element _outactors
      _)))