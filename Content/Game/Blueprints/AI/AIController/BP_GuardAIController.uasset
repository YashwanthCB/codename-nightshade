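; AI controller for patrol guards that runs the BT_PatrolGuard behavior tree and starts awareness in Roaming.
; On possess, it derives a two-point patrol from the guard's spawn location, forward vector and WalkDistance.
; GetGotoLocation returns the start point when the guard is near the far point, otherwise the far point.
; A hearing processor component picks the loudest sound, but sound and perception-loss events only print debug messages.
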(event `self.ReceiveBeginPlay`
  (`NSAIHearingProcessor.InitializeProcessing` (`self.BP_NSAIHearingProcessor`) (`self.AIPerceptionHearing`)))

(event `self.ReceivePossess`
  (params (PossessedPawn :type "Pawn Object Reference"))
  (`self.RunBehaviorTree` "/Game/Game/Blueprints/AI/AIBehaviour/BT_PatrolGuard.BT_PatrolGuard")
  (bind _asbp_ai_patrol_guard (cast `/Game/Game/Blueprints/AI/Character/BP_AI_PatrolGuard` PossessedPawn))
  (bind _output_get (set `self.AI Patrol Guard` _asbp_ai_patrol_guard))
  (bind _returnvalue (`self.K2_GetActorLocation` _output_get))
  (set `self.InitialPawnLocation` _returnvalue)
  (set `self.DestinationLocation` (+ _returnvalue (* (`self.GetActorForwardVector` _output_get) (`/Game/Game/Blueprints/AI/Character/BP_AI_PatrolGuard.WalkDistance` _output_get))))
  (`BlackboardComponent.SetValueAsEnum` (`self.Blackboard`) (`self.AIAwarenessState`) (enumliteral `EAIAwarenessState` "Roaming"))
  (set `self.SwapLocation` (`self.InitialPawnLocation`)))

(event `self.BP_NSAIHearingProcessor.LoudestSoundEvent`
  (params (`Loudest Actor` :type "Actor Object Reference") (`Noise Information` :type "/Game/Game/Blueprints/Environment/AI/FNoiseInformation Structure"))
  (`KismetSystemLibrary.PrintString` (`KismetStringLibrary.Concat_StrStr` (`KismetSystemLibrary.GetDisplayName` self) ": " (`KismetSystemLibrary.GetDisplayName` `Loudest Actor`) ", " (`KismetStringLibrary.Conv_DoubleToString` (`.NoiseIntensity_2_A44C64D148E414DF8CF6C58FD6DC1D2E` (break `/Game/Game/Blueprints/Environment/AI/FNoiseInformation` `Noise Information`)))) false))

(event `self.AIPerceptionHearing.OnTargetPerceptionForgotten`
  (params (Actor :type "Actor Object Reference"))
  (`KismetSystemLibrary.PrintString` "Forgoten in Guard AI controller" true true (struct :`R` 1.0 :`G` 0.226266 :`B` 0.056156 :`A` 1.0)))

(event `self.AIPerceptionHearing.OnTargetPerceptionUpdated`
  (params (Actor :type "Actor Object Reference") (Stimulus :type "AIStimulus Structure"))
  (if (not (`.bSuccessfullySensed` (break `AIStimulus` Stimulus)))
    (`KismetSystemLibrary.PrintString` "Forgoten in Guard AI controller by un sensing" true true (struct :`R` 1.0 :`G` 0.226266 :`B` 0.056156 :`A` 1.0))))

(fn `GetGotoLocation`
  (returns (Location :type "Vector Structure"))
  (locals (ReturnVal :type "Vector Structure"))
  (bind _destinationlocation (`self.DestinationLocation`))
  (bind _returnvalue (`self.K2_GetActorLocation` (`self.K2_GetPawn`)))
  (if (== _returnvalue (`self.DestinationLocation`) :`ErrorTolerance` 50.0)
    (return (`self.InitialPawnLocation`))
    (elif (== _returnvalue (`self.InitialPawnLocation`) :`ErrorTolerance` 50.0)
      (return _destinationlocation)
      (else
        (return _destinationlocation)))))

(fn `GetVisionSenseComponent`
  (returns (ReturnValue :type "VisionSenseComponent Object Reference"))
  (return (`/Game/Game/Blueprints/AI/Character/BP_AI_PatrolGuard.VisionSenseComponent` (`self.AI Patrol Guard`))))

(fn `UserConstructionScript`)