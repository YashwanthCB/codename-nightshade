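; First-person shooter game mode Blueprint that passes mission objective state to the player HUD.
; UpdateUIModel casts the first player controller's HUD to BPPlayerHUD and copies in the title and description of the first mission objective.
; When the objective list is empty, it flags all objectives as complete on the HUD instead.
; Tick only calls its parent implementation.
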(event `self.UpdateUIModel`
  (bind _missionobjectives (`Mission.MissionObjectives` (`self.Mission`)))
  (bind (_missionid _objective _description) (break `MissionObjective` (`|GetArrayItem` _missionobjectives)))
  (bind _asbpplayer_hud (cast `/Game/Game/Blueprints/BPPlayerHUD` (`PlayerController.GetHUD` (`GameplayStatics.GetPlayerController` 0))))
  (if (`KismetArrayLibrary.Array_IsEmpty` _missionobjectives)
    (set `/Game/Game/Blueprints/BPPlayerHUD.AllObjectivesComplete?` true _asbpplayer_hud)
    (else
      (set `/Game/Game/Blueprints/BPPlayerHUD.CurrentObjectiveTitle` _objective _asbpplayer_hud)
      (set `/Game/Game/Blueprints/BPPlayerHUD.CurrentObjectiveDesc` _description _asbpplayer_hud))))

(event `self.ReceiveTick`
  (params (DeltaSeconds :type "Float (single-precision)"))
  (`parent.ReceiveTick` DeltaSeconds))

(fn `UserConstructionScript`)