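; Grapple hook target point that shows a highlight widget while active.
; GrappleDetect overlap events set IsPlayerOverlapping without checking which actor overlaps.
; Activate highlights the point, but during an overlap it deactivates it instead and switches GrappleDetect to WorldStatic, ignoring a custom trace channel.
; End overlap restores blocking on that channel and a custom object type, leaving the highlight for a later Activate call.
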(event `self.GrappleDetect.OnComponentBeginOverlap`
  (params (OverlappedComponent :type "PrimitiveComponent Object Reference") (OtherActor :type "Actor Object Reference") (OtherComp :type "PrimitiveComponent Object Reference") (OtherBodyIndex :type Integer) (bFromSweep :type Boolean) (SweepResult :type "HitResult Structure (by ref)"))
  (set `self.bIsPlayerOverlapping` true))

(event `self.GrappleDetect.OnComponentEndOverlap`
  (params (OverlappedComponent :type "PrimitiveComponent Object Reference") (OtherActor :type "Actor Object Reference") (OtherComp :type "PrimitiveComponent Object Reference") (OtherBodyIndex :type Integer))
  (set `self.bIsPlayerOverlapping` false)
  (`PrimitiveComponent.SetCollisionResponseToChannel` (`self.GrappleDetect`) "ECC_GameTraceChannel4" "ECR_Block")
  (`PrimitiveComponent.SetCollisionObjectType` (`self.GrappleDetect`) "ECC_GameTraceChannel1"))

(fn `Activate`
  (if (not (`self.bIsPlayerOverlapping`))
    (set `self.bIsactive` true)
    (`SceneComponent.SetVisibility` (`self.GrappleHighlightWidget`) true false)
    (else
      (`PrimitiveComponent.SetCollisionResponseToChannel` (`self.GrappleDetect`) "ECC_GameTraceChannel4" "ECR_Ignore")
      (`PrimitiveComponent.SetCollisionObjectType` (`self.GrappleDetect`) "ECC_WorldStatic")
      (`self.Deactivate`))))

(fn `Deactivate`
  (set `self.bIsactive` false)
  (`SceneComponent.SetVisibility` (`self.GrappleHighlightWidget`) false false))

(fn `UserConstructionScript`)