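; Game mode for a hostage-tagging mission that decides when the mission is accomplished.
; On BeginPlay it binds a handler to the OnDoorUnlocked event, which adds to the HostagesTagged count.
; After a short delay, the handler sets MissionAccomplished if that count has reached TotalHostages.
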(event `self.ReceiveBeginPlay`
  (add `self.OnDoorUnlocked` (delegate `On Door Unlocked`)))

(event `On Door Unlocked` :!signature `self.OnDoorUnlocked`
  (params (`Hostages Tagged ` :type Integer))
  (set `self.Hostages Tagged` (+ `Hostages Tagged ` (`self.Hostages Tagged`)))
  (`KismetSystemLibrary.Delay` 2.0)
  (if (>= (`self.Hostages Tagged`) (`self.Total Hostages`))
    (set `self.MissionAccomplished` true)))

(fn `UserConstructionScript`)