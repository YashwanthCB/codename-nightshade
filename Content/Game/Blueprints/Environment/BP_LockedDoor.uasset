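; Locked door that requires a hacking puzzle to be solved before its inherited interaction logic runs.
; BeginPlay creates the puzzle widget and binds to BPPlayerHUD's puzzle events; interacting while unsolved shows it with UI-only input and processing audio.
; The solved event acts only on the activated door, closing the UI, running the parent interaction once and notifying HostageTagGameMode with HostagedBehindTheDoor.
; Later interactions go straight to the parent logic.
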(event `self.ReceiveBeginPlay`
  (bind _asbpplayer_hud (cast `/Game/Game/Blueprints/BPPlayerHUD` (`PlayerController.GetHUD` (`GameplayStatics.GetPlayerController` 0))))
  (add `/Game/Game/Blueprints/BPPlayerHUD.OnPuzzleUIClosed` _asbpplayer_hud (delegate `CloseHackUI`))
  (add `/Game/Game/Blueprints/BPPlayerHUD.OnPuzzleSolved` _asbpplayer_hud (delegate `OnPuzzleSolved_Event`))
  (bind _returnvalue (`|CreateWidget` "/Game/Game/Blueprints/Widgets/PuzzleMechanics/WBP_DoorPuzzleBasic.WBP_DoorPuzzleBasic_C"))
  (set `self.PuzzleWidgetRef` _returnvalue)
  (`AudioMixerBlueprintLibrary.PrimeSoundCueForPlayback` "/Game/Game/Sounds/SFX/button_press_1_Cue.button_press_1_Cue")
  (`AudioMixerBlueprintLibrary.PrimeSoundCueForPlayback` "/Game/Game/Sounds/SFX/computer_processing_Cue.computer_processing_Cue"))

(event `OnPuzzleSolved_Event`
  (if (`self.bIsPuzzleActivated`)
    (`self.CloseHackUI`)
    (`/Engine/EditorBlueprintResources/StandardMacros.DoOnce` false
      (:`Completed`
        (`parent.InteractionLogic` (`self.Target`))
        (set `self.IsPuzzleSolved?` true)
        (bind _ashostage_tag_game_mode (cast `/Game/Game/Blueprints/HostageTagGameMode` (`GameplayStatics.GetGameMode`)))
        (`/Game/Game/Blueprints/HostageTagGameMode.On Door Unlocked` _ashostage_tag_game_mode (`self.HostagedBehindTheDoor`))))))

(event `self.OnInteractionClicked_Event`
  (set `self.bIsPuzzleActivated` true)
  (`UserWidget.AddToViewport` (`self.PuzzleWidgetRef`) 0)
  (bind _returnvalue (`GameplayStatics.GetActorOfClass` (`GameModeBase.PlayerControllerClass` (`GameplayStatics.GetGameMode`))))
  (`WidgetBlueprintLibrary.SetInputMode_UIOnlyEx` _returnvalue null)
  (set `PlayerController.bShowMouseCursor` true _returnvalue)
  (`AudioComponent.Play` (`self.ProcessingSound`) 0.0))

(event `self.InteractionLogic`
  (params (Target :type "Actor Object Reference"))
  (if (`self.IsPuzzleSolved?`)
    (`parent.InteractionLogic` Target)
    (else
      (set `self.Target` Target)
      (`self.OnInteractionClicked_Event`))))

(event `CloseHackUI`
  (bind _returnvalue (`GameplayStatics.GetPlayerController` 0))
  (`AudioComponent.Stop` (`self.ProcessingSound`))
  (`Widget.RemoveFromParent` (`self.PuzzleWidgetRef`))
  (set `self.InitiallyOpen?` true)
  (`WidgetBlueprintLibrary.SetInputMode_GameOnly` _returnvalue)
  (set `PlayerController.bShowMouseCursor` false _returnvalue)
  (set `self.bIsPuzzleActivated` false))

(fn `UserConstructionScript`
  (`parent.UserConstructionScript`))