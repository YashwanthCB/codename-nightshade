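; Noise sensor actor that sounds an alarm and lights a siren when detected noise reaches suspicion or detection intensity.
; Each noise event picks an intensity band that sets the alarm cue's detection type and lerps the siren from yellow toward red.
; The ThresholdTrigger macro blocks drops to a lower alarm level.
; Noise below suspicion starts a one-shot cooldown timer that resets a raised alarm.
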(event `NoiseDetected`
  (params (`Noise Maker` :type "Actor Object Reference") (`Noise Information` :type "/Game/Game/Blueprints/Environment/AI/FNoiseInformation Structure"))
  (bind _noiseintensity (break `/Game/Game/Blueprints/Environment/AI/FNoiseInformation` `Noise Information`))
  (set `self.NoiseIntensity` _noiseintensity)
  (`self.HandleBeeping`)
  (`KismetSystemLibrary.PrintString` (`KismetStringLibrary.Concat_StrStr` (`KismetSystemLibrary.GetDisplayName` self) ": " (`KismetStringLibrary.Conv_DoubleToString` _noiseintensity) "dbdb") false))

(event `HandleBeeping`
  (bind _noiseintensity (`self.NoiseIntensity`))
  (bind _suspicion_intensity (`self.Suspicion Intensity`))
  (bind _detectionintensity (`self.DetectionIntensity`))
  (bind _alarm_sound_cue (`self.alarm_sound_cue`))
  (if (`KismetMathLibrary.InRange_FloatFloat` _noiseintensity 0.0 _suspicion_intensity true false)
    (if (`self.DidAlarmRaise?`)
      (`/Engine/EditorBlueprintResources/StandardMacros.DoOnce` false :!label _label
        (:`Completed`
          (bind _returnvalue (`/Game/Game/Blueprints/FunctionLibrary/BasicLibrary.SetOrResetTimer` 5.0 (delegate `ResetIndicator`) self (`self.TimerHandle`)))
          (set `self.TimerHandle` _returnvalue)))
      (else
        (`AudioComponent.SetIntParameter` _alarm_sound_cue "Detection Type" -1)))
    (elif (`KismetMathLibrary.InRange_FloatFloat` _noiseintensity _suspicion_intensity _detectionintensity true false)
      (`self.ThresholdTrigger` 1
        (:`Out`
          (`AudioComponent.SetIntParameter` _alarm_sound_cue "Detection Type" 0)
          (set `self.DidAlarmRaise?` true)
          (`self.LerpSensorMaterialColor` :!label _label_2)
          (goto _label :!via `Reset`)))
      (elif (`KismetMathLibrary.InRange_FloatFloat` _noiseintensity _detectionintensity 100.0)
        (`self.ThresholdTrigger` 2
          (:`Out`
            (`AudioComponent.SetIntParameter` _alarm_sound_cue "Detection Type" 1)
            (set `self.DidAlarmRaise?` true)
            (goto _label_2)))))))

(event `ResetIndicator`
  (bind _siren (`self.Siren`))
  (`MeshComponent.SetVectorParameterValueOnMaterials` _siren "LightColor" (`KismetMathLibrary.Conv_LinearColorToVector` (struct :`R` 1.0 :`G` 1.0 :`B` 1.0 :`A` 1.0)))
  (`MeshComponent.SetScalarParameterValueOnMaterials` _siren "LightIntensity" 0.0)
  (`AudioComponent.SetIntParameter` (`self.alarm_sound_cue`) "Detection Type" -1)
  (set `self.DidAlarmRaise?` false)
  (set `self.AlarmLevel` 0))

(event `self.ReceiveBeginPlay`
  (bind _siren (`self.Siren`))
  (`MeshComponent.SetVectorParameterValueOnMaterials` _siren "LightColor" (`KismetMathLibrary.Conv_LinearColorToVector` (struct :`R` 1.0 :`G` 1.0 :`B` 1.0 :`A` 1.0)))
  (`MeshComponent.SetScalarParameterValueOnMaterials` _siren "LightIntensity" 0.0))

(fn `LerpSensorMaterialColor`
  (bind _siren (`self.Siren`))
  (`MeshComponent.SetVectorParameterValueOnMaterials` _siren "LightColor" (`KismetMathLibrary.Conv_LinearColorToVector` (`KismetMathLibrary.LinearColorLerp` (struct :`R` 0.917436 :`G` 1.0 :`A` 1.0) (struct :`R` 1.0 :`B` 0.025572 :`A` 1.0) (`KismetMathLibrary.MapRangeClamped` (`self.NoiseIntensity`) (`self.Suspicion Intensity`) 100.0 0.0 1.0))))
  (`MeshComponent.SetScalarParameterValueOnMaterials` _siren "LightIntensity" 100.0))

(fn `UserConstructionScript`)