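; BP_SimpleDoor is an interactable door, but its opening logic is disconnected in this graph.
; BeginPlay primes the open sound and copies InitiallyOpen into IsOpen, while interaction forwards to an empty InteractionLogic event.
; FixDoor and the construction script are also empty.
; Unwired nodes hold rotation toggling that picks swing direction from a forward-vector dot product and spawns a disturbance indicator whenever the door differs from its initial state.
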(event `self.ReceiveBeginPlay`
  (`AudioMixerBlueprintLibrary.PrimeSoundCueForPlayback` "/Game/Game/Sounds/SFX/door_open_Cue.door_open_Cue")
  (set `self.IsOpen` (`self.InitiallyOpen?`)))

(event `BPInteract_1`
  (params (InInstigator :type "Actor Object Reference"))
  (`self.InteractionLogic` InInstigator))

(event `InteractionLogic`
  (params (Target :type "Actor Object Reference")))

(event `FixDoor_1`
  (params (InAIController :type "AIController Object Reference")))

(fn `UserConstructionScript`)