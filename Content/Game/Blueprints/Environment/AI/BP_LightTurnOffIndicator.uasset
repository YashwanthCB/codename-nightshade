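; BP_LightTurnOffIndicator is an environment actor that displays the current light exposure measured on it as text.
; On BeginPlay it runs the parent logic, then registers its BoxCollision as the component ConstantLightInfluence checks for hits.
; Every Tick it writes the exposure value from ConstantLightInfluence to its TextRender.
; GetLightInfluenceComponent exposes that influence component to callers.
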(event `self.ReceiveBeginPlay`
  (`parent.ReceiveBeginPlay`)
  (`LightInfluenceComponent.SetComponentToCheckHit` (`self.ConstantLightInfluence`) (`self.BoxCollision`)))

(event `self.ReceiveTick`
  (params (DeltaSeconds :type "Float (single-precision)"))
  (`TextRenderComponent.K2_SetText` (`self.TextRender`) (`KismetTextLibrary.Conv_StringToText` (`KismetStringLibrary.Concat_StrStr` "light exposure: " (`KismetStringLibrary.Conv_DoubleToString` (`LightInfluenceComponent.GetLightExposure` (`self.ConstantLightInfluence`)))))))

(fn `GetLightInfluenceComponent`
  (returns (ReturnValue :type "LightInfluenceComponent Object Reference"))
  (return (`self.ConstantLightInfluence`)))

(fn `UserConstructionScript`)