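; AI hearing processor component that picks out the loudest noise an AI-controlled pawn perceives.
; Hearing perception updates store each source actor's tag and intensity, attenuated through all mediums, in a noise map, removing actors when sensing fails or they are forgotten.
; When dispatching is enabled, Tick broadcasts the loudest entry if it meets a fixed threshold, then clears the map.
; A getter also exposes the loudest actor, intensity and tag.
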(event `self.ReceiveInitializeProcessing`
  (add `AIPerceptionComponent.OnTargetPerceptionUpdated` (`self.AIPerceptionHearingComponent`) (delegate `OnTargetPerceptionUpdated_Event`))
  (add `AIPerceptionComponent.OnTargetPerceptionForgotten` (`self.AIPerceptionHearingComponent`) (delegate `OnTargetPerceptionForgotten_Event`)))

(event `OnTargetPerceptionForgotten_Event`
  (params (Actor :type "Actor Object Reference"))
  (`BlueprintMapLibrary.Map_Remove` (`self.ActorNoiseMap`) Actor))

(event `OnTargetPerceptionUpdated_Event`
  (params (Actor :type "Actor Object Reference") (Stimulus :type "AIStimulus Structure"))
  (bind (_age _expirationage _strength _stimuluslocation _receiverlocation _tag _bsuccessfullysensed) (break `AIStimulus` Stimulus))
  (bind _actornoisemap (`self.ActorNoiseMap`))
  (if _bsuccessfullysensed
    (`BlueprintMapLibrary.Map_Add` _actornoisemap Actor (make `/Game/Game/Blueprints/Environment/AI/FNoiseInformation` (`/Game/Game/Blueprints/FunctionLibrary/BasicLibrary.AttenuateSoundThroughAllMediums` (`Controller.K2_GetPawn` (cast `AIController` (`self.GetOwner`) :!pure true)) Actor Stimulus (`self.HearingRange`)) _tag))
    (else
      (`BlueprintMapLibrary.Map_Remove` _actornoisemap Actor))))

(event `self.ReceiveTick`
  (params (DeltaSeconds :type "Float (single-precision)"))
  (bind (_actor _loudest_noise_information) (`self.GetLoudestSoundingActorBP`))
  (if (`self.DispatchLoudestSound?`)
    (if (>= (`.NoiseIntensity_2_A44C64D148E414DF8CF6C58FD6DC1D2E` (break `/Game/Game/Blueprints/Environment/AI/FNoiseInformation` _loudest_noise_information)) 25.0)
      (`self.LoudestSoundEvent` _actor _loudest_noise_information)
      (`BlueprintMapLibrary.Map_Clear` (`self.ActorNoiseMap`)))))

(fn `GetLoudestSoundingActor`
  (returns (OutActor :type "Actor Object Reference") (Sound :type "Float (single-precision)") (OutTag :type Name) (ReturnValue :type Boolean))
  (bind (_actor _loudest_noise_information) (`self.GetLoudestSoundingActorBP`))
  (bind (_noiseintensity _tag) (break `/Game/Game/Blueprints/Environment/AI/FNoiseInformation` _loudest_noise_information))
  (return _actor _noiseintensity _tag (`KismetSystemLibrary.IsValid` _actor)))

(fn `GetLoudestSoundingActorBP`
  (returns (Actor :type "Actor Object Reference") (`Loudest Noise Information` :type "/Game/Game/Blueprints/Environment/AI/FNoiseInformation Structure"))
  (locals (Max :type "Float (double-precision)") (IndexForMax :type Integer) (Max1 :type "/Game/Game/Blueprints/Environment/AI/FNoiseInformation Structure"))
  (bind _values (`BlueprintMapLibrary.Map_Values` (`self.ActorNoiseMap`)))
  (for (_array_element _array_index) _values
    (if (>= (`.NoiseIntensity_2_A44C64D148E414DF8CF6C58FD6DC1D2E` (break `/Game/Game/Blueprints/Environment/AI/FNoiseInformation` _array_element)) (`.NoiseIntensity_2_A44C64D148E414DF8CF6C58FD6DC1D2E` (break `/Game/Game/Blueprints/Environment/AI/FNoiseInformation` (`local.Max1`))))
      (set `local.Max1` _array_element)
      (set `local.IndexForMax` _array_index)))
  (bind _keys (`BlueprintMapLibrary.Map_Keys` (`self.ActorNoiseMap`)))
  (return (`|GetArrayItem` _keys (`local.IndexForMax`)) (`local.Max1`)))