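; Blueprint function library with a timer-restart helper and functions that compute how loud an AI hearing stimulus is at its receiver.
; Distance attenuation subtracts a linearly mapped, clamped loss from strength, floored at zero, and returns zero beyond hearing range.
; The through-medium variants multi-trace from source to receiver, reapplying full-path air loss plus an obstacle penalty per hit, then air loss again.
; The Single variant uses another trace channel and penalizes only the first hit.
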(fn `AttenuateSound`
  (params (WorldContextObject :type "Object Object Reference") (Stimulus :type "AIStimulus Structure") (HearingRange :type "Float (double-precision)"))
  (returns (`Attenuated Sound` :type "Float (double-precision)"))
  (bind (_age _expirationage _strength _stimuluslocation _receiverlocation) (break `AIStimulus` Stimulus))
  (bind _returnvalue (`KismetMathLibrary.Vector_Distance` _stimuluslocation _receiverlocation))
  (if (>= _returnvalue HearingRange)
    (return 0.0)
    (else
      (return (`KismetMathLibrary.FMax` (- _strength (`KismetMathLibrary.MapRangeClamped` _returnvalue 10000.0 0.0 100.0 0.0)))))))

(fn `AttenuateSoundInAir`
  (params (HearingRange :type "Float (double-precision)") (Strength :type "Float (double-precision)") (`Sound Source` :type "Vector Structure") (`Sound Slot Start` :type "Vector Structure") (`Sound Slot End` :type "Vector Structure"))
  (returns (`Attenuated Sound` :type "Float (double-precision)"))
  (if (>= (`KismetMathLibrary.Vector_Distance` `Sound Source` `Sound Slot End`) HearingRange)
    (return 0.0)
    (else
      (return (`KismetMathLibrary.FMax` (- Strength (`KismetMathLibrary.MapRangeClamped` (`KismetMathLibrary.Vector_Distance` `Sound Slot Start` `Sound Slot End`) 10000.0 0.0 100.0 0.0)))))))

(fn `AttenuateSoundThroughAllMediums`
  (params (WorldContextObject :type "Object Object Reference") (StimulatingActor :type "Actor Object Reference") (Stimulus :type "AIStimulus Structure") (HearingRange :type "Float (double-precision)"))
  (returns (`Attenuated Sound` :type "Float (double-precision)"))
  (locals (`Actor Names` :type String :default "MultiLineTrace: ") (AttenuatedSound :type "Float (double-precision)" :default 0.0) (`Sound to reduce` :type "Float (double-precision)" :default 40.0))
  (bind (_age _expirationage _strength _stimuluslocation _receiverlocation) (break `AIStimulus` Stimulus))
  (set `local.AttenuatedSound` _strength)
  (bind _outhits (`KismetSystemLibrary.LineTraceMulti` WorldContextObject _stimuluslocation _receiverlocation "TraceTypeQuery5" false (`|MakeArray` StimulatingActor) "ForDuration" true (struct :`R` 1.0 :`A` 1.0) (struct :`G` 1.0 :`A` 1.0) 40.0))
  (for _ _outhits
    (bind _output_get (set `local.AttenuatedSound` (`self.AttenuateSoundInAir` HearingRange (`local.AttenuatedSound`) _stimuluslocation _stimuluslocation _receiverlocation WorldContextObject)))
    (set `local.AttenuatedSound` (- _output_get (`local.Sound to reduce`))))
  (set `local.AttenuatedSound` (`self.AttenuateSoundInAir` HearingRange (`local.AttenuatedSound`) _stimuluslocation _stimuluslocation _receiverlocation WorldContextObject))
  (`KismetSystemLibrary.PrintString` WorldContextObject (`KismetStringLibrary.Concat_StrStr` " produces " (`KismetStringLibrary.Conv_DoubleToString` (`local.AttenuatedSound`)) " db") false)
  (return (`local.AttenuatedSound`)))

(fn `AttenuateSoundThroughAllMediumsSingle`
  (params (WorldContextObject :type "Object Object Reference") (StimulatingActor :type "Actor Object Reference") (Stimulus :type "AIStimulus Structure") (HearingRange :type "Float (double-precision)"))
  (returns (`Attenuated Sound` :type "Float (double-precision)"))
  (locals (`Actor Names` :type String :default "MultiLineTrace: ") (AttenuatedSound :type "Float (double-precision)"))
  (bind (_age _expirationage _strength _stimuluslocation _receiverlocation) (break `AIStimulus` Stimulus))
  (set `local.AttenuatedSound` _strength)
  (bind _outhits (`KismetSystemLibrary.LineTraceMulti` WorldContextObject _stimuluslocation _receiverlocation "TraceTypeQuery6" false (`|MakeArray` StimulatingActor) "ForDuration" true (struct :`R` 1.0 :`A` 1.0) (struct :`G` 1.0 :`A` 1.0) 40.0))
  (for _array_element _outhits
    (bind _output_get (set `local.AttenuatedSound` (`self.AttenuateSoundInAir` HearingRange (`local.AttenuatedSound`) _stimuluslocation _stimuluslocation _receiverlocation WorldContextObject)))
    (set `local.AttenuatedSound` (- _output_get 40.0))
    (bind (_bblockinghit _binitialoverlap _time _distance _location _impactpoint _normal _impactnormal _physmat _hitactor) (`GameplayStatics.BreakHitResult` _array_element))
    (`KismetSystemLibrary.PrintString` _hitactor (`KismetSystemLibrary.GetDisplayName` _hitactor))
    (break))
  (set `local.AttenuatedSound` (`self.AttenuateSoundInAir` HearingRange (`local.AttenuatedSound`) _stimuluslocation _stimuluslocation _receiverlocation WorldContextObject))
  (return (`local.AttenuatedSound`)))

(fn `SetOrResetTimer`
  (params (CooldownTimer :type "Float (double-precision)") (TimerCallback :type Delegate) (WorldContextObject :type "Object Object Reference") (`Timer Handle` :type "TimerHandle Structure"))
  (returns (ReturnValue :type "TimerHandle Structure"))
  (if (`KismetSystemLibrary.K2_IsTimerActiveHandle` WorldContextObject `Timer Handle`)
    (`KismetSystemLibrary.K2_ClearAndInvalidateTimerHandle` WorldContextObject `Timer Handle`) ; Clear existing timer handle
  )
  (bind _returnvalue (`KismetSystemLibrary.K2_SetTimerDelegate` TimerCallback CooldownTimer)) ; Create a new timer
  (return _returnvalue))