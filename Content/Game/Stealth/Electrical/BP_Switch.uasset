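; BP_Switch is an interactable electrical switch in the Stealth folder whose button glows green when on and red when off.
; On BeginPlay, after the parent logic, and on each BPInteract, it passes IsTurnedOn to HandleButtonMaterials, which sets the Glow Color parameter on the button mesh's materials.
; The Blueprint only handles this visual feedback and never changes IsTurnedOn itself.
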(event `self.ReceiveBeginPlay`
  (`parent.ReceiveBeginPlay`)
  (`self.HandleButtonMaterials` (`self.IsTurnedOn`)))

(event `self.BPInteract`
  (params (InInstigator :type "Actor Object Reference"))
  (`self.HandleButtonMaterials` (`self.IsTurnedOn`)))

(fn `HandleButtonMaterials`
  (params (`IsTurnedOn?` :type Boolean))
  (bind _buttonstaticmesh (`self.ButtonStaticMesh`))
  (if `IsTurnedOn?`
    (`MeshComponent.SetVectorParameterValueOnMaterials` _buttonstaticmesh "Glow Color" (`KismetMathLibrary.Conv_LinearColorToVector` (`KismetMathLibrary.LinearColor_Green`)))
    (else
      (`MeshComponent.SetVectorParameterValueOnMaterials` _buttonstaticmesh "Glow Color" (`KismetMathLibrary.Conv_LinearColorToVector` (`KismetMathLibrary.LinearColor_Red`))))))

(fn `UserConstructionScript`)